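; First-person player character handling movement, look, jump, crouch, sprint, health, stamina and inventory input.
; BeginPlay creates the in-game UI widget, whose inventory menu toggles with the cursor, while Interact calls item pickup below five items.
; Tick regenerates health, updates UI values and uses Delays to throttle stamina drain and recovery, forcing walk speed at zero.
; Dropped items are unhidden with collision restored, but their transform move is unwired.
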(event `InputAction|Inventory`
  (params (Key :type "Key Structure" :default "AnyKey"))
  (bind _character_ui_reference_ingame (`self.Character_UI_Reference_InGame`))
  (bind _inventorymenu (`/Game/Assets/Blueprints/inGameUI.InventoryMenu` _character_ui_reference_ingame))
  (:`Pressed`
    (if (`/Game/Assets/Blueprints/inGameUI.Inventory_Active` _character_ui_reference_ingame)
      (`/Engine/EditorBlueprintResources/StandardMacros.FlipFlop`
        (:`A`
          (`Widget.SetVisibility` _inventorymenu "Visible")
          (set `self.Character_Inventory_Open` true)
          (`self.Character_UI_Cursor_Show`))
        (:`B`
          (`Widget.SetVisibility` _inventorymenu "Hidden")
          (set `self.Character_Inventory_Open` false)
          (`self.Character_UI_Cursor_Hide`))))))

(event `InputAction|Sprint`
  (params (Key :type "Key Structure" :default "AnyKey"))
  (:`Pressed`
    (`|ExecutionSequence`
      (:`then_0`
        (`self.Character_Input_Sprint` true))))
  (:`Released`
    (`|ExecutionSequence`
      (:`then_0`
        (`self.Character_Input_Sprint` false)))))

(event `self.ReceiveBeginPlay`
  (`|ExecutionSequence`
    (:`then_0`
      (`self.Character_Init_Hud`))))

(event `InputAction|Crouch`
  (params (Key :type "Key Structure" :default "AnyKey"))
  (:`Pressed`
    (`|ExecutionSequence`
      (:`then_0`
        (`self.Character_Input_Crouch` true))))
  (:`Released`
    (`|ExecutionSequence`
      (:`then_0`
        (`self.Character_Input_Crouch` false)))))

(event `InputAxis|Turn`
  (params (AxisValue :type "Float (single-precision)"))
  (`|ExecutionSequence`
    (:`then_0`
      (`self.Character_Input_Mouse_Turn` AxisValue))))

(event `InputAxis|LookUp`
  (params (AxisValue :type "Float (single-precision)"))
  (`|ExecutionSequence`
    (:`then_0`
      (`self.Character_Input_Mouse_Look` AxisValue))))

(event `InputAction|Jump`
  (params (Key :type "Key Structure" :default "AnyKey"))
  (:`Pressed`
    (`|ExecutionSequence`
      (:`then_0`
        (`self.Character_Input_Jump` true))))
  (:`Released`
    (`|ExecutionSequence`
      (:`then_0`
        (`self.Character_Input_Jump` false)))))

(event `InputAxis|MoveForward`
  (params (AxisValue :type "Float (single-precision)"))
  (`|ExecutionSequence`
    (:`then_0`
      (`self.Character_Input_Movement_Forward` AxisValue))))

(event `InputAxis|MoveRight`
  (params (AxisValue :type "Float (single-precision)"))
  (`|ExecutionSequence`
    (:`then_0`
      (`self.Character_Input_Movement_Right` AxisValue))))

(event `self.ReceiveTick`
  (params (DeltaSeconds :type "Float (single-precision)"))
  (bind _character_stamina_max (`self.Character_Stamina_Max`))
  (bind _character_stamina_value (`self.Character_Stamina_Value`))
  (`|ExecutionSequence`
    (:`then_0`
      (`|ExecutionSequence`
        (:`then_0`
          (set `self.Character_UI_Value_Stamina` (/ (`self.Character_Stamina_Value`) 100.0)))
        (:`then_1`
          (if (and (`self.Character_Key_Sprint_Down`) (> (`KismetMathLibrary.VSize` (`MovementComponent.Velocity` (`self.CharacterMovement`))) 210.0) (not (`self.Character_isCrouched`)))
            (`KismetSystemLibrary.Delay` 0.06)
            (set `self.Character_Stamina_Value` (`KismetMathLibrary.FClamp` (- _character_stamina_value (`self.Character_Stamina_Depletion_Rate`)) 0.0 _character_stamina_max))
            (else
              (`KismetSystemLibrary.Delay` 0.35)
              (set `self.Character_Stamina_Value` (`KismetMathLibrary.FClamp` (+ _character_stamina_value (`self.Character_Stamina_Recover_Rate`)) 0.0 _character_stamina_max))))
          (if (== (`KismetMathLibrary.FTrunc` _character_stamina_value) 0)
            (set `self.Character_Sprint_Can_Run` false)
            (set `self.Character_Sprint_isRunning` false)
            (set `CharacterMovementComponent.MaxWalkSpeed` (`self.Character_Movement_WalkSpeed`) (`self.CharacterMovement`))
            (else
              (set `self.Character_Sprint_Can_Run` true))))))
    (:`then_1`
      (set `self.Character_UI_Value_Health` (/ (`self.Character_Health_Value`) 100.0)))
    (:`then_2`
      (`self.Character_Health_Regen`))))

(event `InputAction|Interact`
  (params (Key :type "Key Structure" :default "AnyKey"))
  (:`Pressed`
    (if (< (`KismetArrayLibrary.Array_Length` (`/Game/Assets/Blueprints/inGameUI.Inventory` (`self.Character_UI_Reference_InGame`))) 5)
      (`self.PickUp_Item`))))

(event `/Game/Assets/Blueprints/Inventory_Action_Interface.Inventory_Action_Item_Drop`
  (params (Inventory_Dropped_Actor :type "Actor Object Reference"))
  (`self.SetActorHiddenInGame` Inventory_Dropped_Actor false)
  (`self.SetActorEnableCollision` Inventory_Dropped_Actor true))

(fn `Character_Health_Regen`
  (if (`self.Character_Health_CanHeal`)
    (set `self.Character_Health_Value` (`KismetMathLibrary.FClamp` (+ (`self.Character_Health_Value`) (`self.Character_Health_RegenRate`)) 0.0 (`self.Character_Health_Max`)))))

(fn `Character_Init_Hud`
  (`|ExecutionSequence`
    (:`then_0`
      (bind _returnvalue (`|CreateWidget` "/Game/Assets/Blueprints/inGameUI.inGameUI_C"))
      (bind _output_get (set `self.Character_UI_Reference_InGame` _returnvalue))
      (`UserWidget.AddToViewport` _output_get 0))))

(fn `Character_Input_Crouch`
  (params (Condition :type Boolean))
  (bind _character_camera_1st (`self.Character_Camera_1st`))
  (if Condition
    (`self.Crouch`)
    (set `self.Character_isCrouched` true)
    (`SceneComponent.K2_SetRelativeLocation` _character_camera_1st (`self.Character_Crouch_Camera_Height`) false false)
    (else
      (`self.UnCrouch`)
      (set `self.Character_isCrouched` false)
      (`SceneComponent.K2_SetRelativeLocation` _character_camera_1st (`self.Character_Crouch_Camera_Default_Height`) false false))))

(fn `Character_Input_Jump`
  (params (Condition :type Boolean))
  (if Condition
    (`self.Jump`)
    (else
      (`self.StopJumping`))))

(fn `Character_Input_Mouse_Look`
  (params (Val :type "Float (double-precision)") (Target :type "Pawn Object Reference"))
  (`self.AddControllerPitchInput` Val))

(fn `Character_Input_Mouse_Turn`
  (params (Val :type "Float (double-precision)"))
  (`self.AddControllerYawInput` Val))

(fn `Character_Input_Movement_Forward`
  (params (ScaleValue :type "Float (double-precision)"))
  (`self.AddMovementInput` (`self.GetActorForwardVector`) ScaleValue))

(fn `Character_Input_Movement_Right`
  (params (ScaleValue :type "Float (double-precision)"))
  (`self.AddMovementInput` (`self.GetActorRightVector`) ScaleValue))

(fn `Character_Input_Sprint`
  (params (Condition :type Boolean))
  (bind _charactermovement (`self.CharacterMovement`))
  (bind _output_get (set `self.Character_Key_Sprint_Down` Condition))
  (if _output_get
    (if (and (`self.Character_Sprint_Can_Run`) (not (`self.Character_isCrouched`)))
      (set `self.Character_Sprint_isRunning` true)
      (set `CharacterMovementComponent.MaxWalkSpeed` (`self.Character_Movement_RunSpeed`) _charactermovement))
    (else
      (set `self.Character_Sprint_isRunning` false)
      (set `CharacterMovementComponent.MaxWalkSpeed` (`self.Character_Movement_WalkSpeed`) _charactermovement)))
  (return))

(fn `Character_Inventory_Refresh`
  (set `self.Character_Inventory_Active` true))

(fn `Character_UI_Cursor_Hide`
  (set `PlayerController.bShowMouseCursor` false (`GameplayStatics.GetPlayerController` 0)))

(fn `Character_UI_Cursor_Show`
  (set `PlayerController.bShowMouseCursor` true (`GameplayStatics.GetPlayerController` 0)))

(fn `UserConstructionScript`)