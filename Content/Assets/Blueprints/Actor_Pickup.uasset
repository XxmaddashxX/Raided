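; Base pickup actor for world items that the player can collect into the inventory.
; The construction script fills the item struct from its image and text variables and applies a custom mesh.
; A trigger toggles the prompt widget and in-range flag for MainCharacter, whose pickup dispatcher the actor binds on BeginPlay.
; On pickup it adds the struct to the UI's inventory, refreshes it, and hides itself with collision disabled rather than being destroyed.
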(event `self.ReceiveBeginPlay`
  (bind _inventory_item_info (`self.Inventory_Item_Info`))
  (bind (_inventory_item_actor _inventory_item_thumbnail _inventory_item_pickuptext) (break `/Game/Assets/Blueprints/Inventory_Structure` _inventory_item_info))
  (bind _returnvalue (`|CreateWidget` "/Game/Assets/Blueprints/hud/PickupActorText.PickupActorText_C"))
  (bind _output_get (set `self.Pickup_Text_Widget` _returnvalue))
  (set `/Game/Assets/Blueprints/hud/PickupActorText.PickupActor` _inventory_item_actor _output_get)
  (set `/Game/Assets/Blueprints/hud/PickupActorText.Pickuptext` _inventory_item_pickuptext _output_get)
  (setmembers `/Game/Assets/Blueprints/Inventory_Structure` :`StructRef` _inventory_item_info :`Inventory_Item_Actor` self)
  (bind _asmain_character (cast `/Game/Assets/Blueprints/MainCharacter` (`GameplayStatics.GetPlayerCharacter` 0)))
  (set `self.MainCharacter` _asmain_character)
  (add `/Game/Assets/Blueprints/MainCharacter.PickUp_Item` _asmain_character (delegate `PickUp_Item_Event_0`)))

(event `PickUp_Item_Event_0`
  (bind _character_ui_reference_ingame (`/Game/Assets/Blueprints/MainCharacter.Character_UI_Reference_InGame` (`self.MainCharacter`)))
  (if (and (`self.IsInRange`) (`self.GetActorEnableCollision`))
    (`KismetArrayLibrary.Array_Add` (`/Game/Assets/Blueprints/inGameUI.Inventory` _character_ui_reference_ingame) (`self.Inventory_Item_Info`))
    (`Widget.RemoveFromParent` (`self.Pickup_Text_Widget`))
    (`self.SetActorHiddenInGame` true)
    (`self.SetActorEnableCollision` false)
    (`/Game/Assets/Blueprints/inGameUI.Refresh Inventory` _character_ui_reference_ingame)))

(event `self.Trigger.OnComponentBeginOverlap`
  (params (OtherActor :type "Actor Object Reference") (OtherComp :type "PrimitiveComponent Object Reference") (OtherBodyIndex :type Integer) (bFromSweep :type Boolean) (SweepResult :type "HitResult Structure (by ref)"))
  (cast `/Game/Assets/Blueprints/MainCharacter` OtherActor)
  (`UserWidget.AddToViewport` (`self.Pickup_Text_Widget`) 0)
  (set `self.IsInRange` true))

(event `self.Trigger.OnComponentEndOverlap`
  (params (OtherActor :type "Actor Object Reference") (OtherComp :type "PrimitiveComponent Object Reference") (OtherBodyIndex :type Integer))
  (cast `/Game/Assets/Blueprints/MainCharacter` OtherActor)
  (`Widget.RemoveFromParent` (`self.Pickup_Text_Widget`))
  (set `self.IsInRange` false))

(fn `UserConstructionScript`
  (setmembers `/Game/Assets/Blueprints/Inventory_Structure` :`StructRef` (`self.Inventory_Item_Info`) :`Inventory_Item_Actor` self :`Inventory_Item_Thumbnail` (`self.InventoryImage`) :`Inventory_Item_PickupText` (`self.PickupText`) :`Inventory_Item_MenuText` (`self.ActionText`))
  (`StaticMeshComponent.SetStaticMesh` (`self.Item`) (`self.CustomMesh`)))